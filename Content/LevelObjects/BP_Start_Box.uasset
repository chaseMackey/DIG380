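; BP_Start_Box is a level-object trigger that damages the first-person character and sends them to a set position.
; On box overlap it subtracts a fixed amount of Health and updates the character's health bar.
; At zero health or below it reloads the current level.
; Otherwise it teleports the character to ToPos, converting the location from actor-local space but applying rotation directly, and prints the health loss.
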(event `self.Box.OnComponentBeginOverlap`
  (params (OverlappedComponent :type "PrimitiveComponent Object Reference") (OtherActor :type "Actor Object Reference") (OtherComp :type "PrimitiveComponent Object Reference") (OtherBodyIndex :type Integer) (bFromSweep :type Boolean) (SweepResult :type "HitResult Structure (by ref)"))
  (bind (_topos_location _topos_rotation) (`KismetMathLibrary.BreakTransform` (`self.ToPos`)))
  (bind _asbp_first_person_character (cast `/Game/FirstPerson/Blueprints/BP_FirstPersonCharacter` OtherActor))
  (bind _output_get (set `/Game/FirstPerson/Blueprints/BP_FirstPersonCharacter.Health` (- (`/Game/FirstPerson/Blueprints/BP_FirstPersonCharacter.Health` _asbp_first_person_character) 20.0) _asbp_first_person_character))
  (`/Game/UI/WBP_Health_Bar.Update Health Bar` (`/Game/FirstPerson/Blueprints/BP_FirstPersonCharacter.Health Bar Refrence` _asbp_first_person_character) _output_get)
  (if (<= (`/Game/FirstPerson/Blueprints/BP_FirstPersonCharacter.Health` _asbp_first_person_character) 0.0)
    (bind _returnvalue (`GameplayStatics.GetCurrentLevelName` true))
    (`GameplayStatics.OpenLevel` (`KismetStringLibrary.Conv_StringToName` _returnvalue))
    (else
      (`self.K2_SetActorLocationAndRotation` _asbp_first_person_character (`KismetMathLibrary.TransformLocation` (`self.GetTransform`) _topos_location) _topos_rotation false false)
      (`KismetSystemLibrary.PrintString` "-20 Health"))))

(fn `UserConstructionScript`)